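; Character component that plays footstep effects, sounds, foley and footprint decals, removing itself when footsteps are disabled.
; Footstep line-traces at the foot socket and maps the physical surface to a data asset that picks Niagara (or Cascade fallback), random audio and footprint tint.
; Gameplay tags select the footprint and foley sets.
; Assets load asynchronously, volume scales with movement speed, and debug mode adds an on-screen widget.
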(event Custom|SpawnNiagara
  (params (Location :type Vector) (PrimaryData :type Primary%20Data%20Asset%20Object%20Reference))
  (bind _surfacedata (N00d|Footsteps|Casting|ConverttoDefaultSurface PrimaryData))
  (bind _overridematerials (Variables|/n00dFootsteps/Core/PDA_N00dFootstepsSurface.PDA_N00dFootstepsSurface_C|GetOverrideMaterials _surfacedata))
  ;[1 1 1] Spawn niagara
  (bind _object (Utilities|AsyncLoadAsset (Variables|/n00dFootsteps/Core/PDA_N00dFootstepsSurface.PDA_N00dFootstepsSurface_C|GetNiagaraEffect (N00d|Footsteps|Casting|ConverttoDefaultSurface PrimaryData)))
    (:Completed
      (bind _asniagara_system (Utilities|Casting|CastToNiagaraSystem _object))
      (bind _returnvalue (Niagara|SpawnSystematLocation _asniagara_system Location))
      ;;[1 1 1] Set materials
      (Utilities|IsValid _returnvalue
        (:Is%20Valid
          (if (Utilities|Array|IsValidIndex _overridematerials)
            (for (_array_element _array_index) _overridematerials
              (Rendering|Material|SetMaterial _returnvalue _array_index _array_element))))))))

(event Custom|SpawnCascade
  (params (Location :type Vector) (PrimaryData :type Primary%20Data%20Asset%20Object%20Reference))
  (bind _surfacedata (N00d|Footsteps|Casting|ConverttoDefaultSurface PrimaryData))
  (bind _overridematerials (Variables|/n00dFootsteps/Core/PDA_N00dFootstepsSurface.PDA_N00dFootstepsSurface_C|GetOverrideMaterials _surfacedata))
  ;[1 1 1] Spawn cascade
  (bind _object (Utilities|AsyncLoadAsset (Variables|/n00dFootsteps/Core/PDA_N00dFootstepsSurface.PDA_N00dFootstepsSurface_C|GetCascadeEffect (N00d|Footsteps|Casting|ConverttoDefaultSurface PrimaryData)))
    (:Completed
      (bind _asparticle_system (Utilities|Casting|CastToParticleSystem _object))
      (bind _returnvalue (Effects|SpawnEmitteratLocation _asparticle_system Location))
      ;;[1 1 1] Set materials
      (Utilities|IsValid _returnvalue
        (:Is%20Valid
          (if (Utilities|Array|IsValidIndex _overridematerials)
            (for (_array_element _array_index) _overridematerials
              (Rendering|Material|SetMaterial _returnvalue _array_index _array_element))))))))

(event Custom|SpawnFoley
  (params (Location :type Vector) (PrimaryData :type Primary%20Data%20Asset%20Object%20Reference))
  ;[1 1 1] Spawn wave
  (bind _object (Utilities|AsyncLoadAsset (.OutItem (Utilities|Array|Random (Variables|/n00dFootsteps/Core/PDA_N00dFootstepsFoley.PDA_N00dFootstepsFoley_C|GetWaves (N00d|Footsteps|Casting|ConverttoDefaultFoley PrimaryData)))))
    (:Completed
      (bind _assound_base (Utilities|Casting|CastToSoundBase _object))
      (bind _returnvalue (Audio|SpawnSoundatLocation _assound_base Location "0, 0, 0" (.Volume (N00d|Footsteps|System|GetVolume)) 1.0 0.0 0 0))
      ;[1 1 1] Bind to completed audio
      (Utilities|IsValid _returnvalue
        (:Is%20Valid
          (EventDispatchers|BindEventtoOnAudioFinished _returnvalue (EventDispatchers|CreateEvent :!event Custom|FoleyAudioFinished))
          ;[1 1 1] Add the incoming and show the int we've added
          (bind _returnvalue_2 (Utilities|Array|Add (Variables|Reference|GetActiveFoleyComponents) 0))
          (Variables|UI|SetActiveFoleyDisplay (Utilities|Text|ToText(Integer) _returnvalue_2)))))))

(event Custom|SpawnFootprint
  (params (Footprint :type FN00d%20Footprint%20Structure%20%28by%20ref%29) (Location :type Vector) (Tint :type Linear%20Color%20Structure))
  (bind (_socket _size _lifetime _opacity _fade _duration _print) (Utilities|Struct|BreakFN00dFootprint Footprint))
  ;[1 1 1] Spawn footprint
  (bind _object (Utilities|AsyncLoadAsset _print)
    (:Completed
      (bind _asmaterial_interface (Utilities|Casting|CastToMaterialInterface _object))
      (bind _returnvalue (Rendering|Decal|SpawnDecalatLocation _asmaterial_interface (Math|Vector|MakeVector _size _size _size) Location (Math|Rotator|MakeRotator 0.0 -9e+01 (+ (.yaw (Transformation|GetActorRotation (N00d|Footsteps|System|GetOwningCharacter))) 9e+01)) _lifetime))
      (Utilities|IsValid _returnvalue
        (:Is%20Valid
          (Variables|UI|SetSocketDisplay (Utilities|Text|ToText(Name) _socket))
          ;[1 1 1] Create MID
          (Rendering|Components|Decal|SetFadeOut _returnvalue _fade _duration true)
          (bind _returnvalue_2 (Rendering|Material|CreateDynamicMaterialInstance (Class|DecalComponent|GetDecalMaterial _returnvalue) "None" "None" :!class /Script/Engine.KismetMaterialLibrary))
          ;[1 1 1] Set the material on the decal and scale the opacity parameter
          (Rendering|Components|Decal|SetDecalMaterial _returnvalue _returnvalue_2)
          (Rendering|Material|SetScalarParameterValue _returnvalue_2 "Opacity" _opacity :!class /Script/Engine.MaterialInstanceDynamic)
          ;[1 1 1] Colour
          (Rendering|Material|SetVectorParameterValue _returnvalue_2 "Colour" Tint :!class /Script/Engine.MaterialInstanceDynamic))))))

(event Custom|FoleyAudioFinished
  (bind _activefoleycomponents (Variables|Reference|GetActiveFoleyComponents))
  ;[1 1 1] Audio finished
  ;;[1 1 1] Remove a sound and debug the active sounds
  (Utilities|Array|RemoveIndex _activefoleycomponents)
  (Variables|UI|SetActiveFoleyDisplay (Utilities|Text|ToText(Integer) (Utilities|Array|Length _activefoleycomponents))))

(event Custom|SpawnAudio
  (params (Location :type Vector) (PrimaryData :type Primary%20Data%20Asset%20Object%20Reference))
  (bind (_volume _speed) (N00d|Footsteps|System|GetVolume))
  ;[1 1 1] Spawn wave
  (bind _object (Utilities|AsyncLoadAsset (.OutItem (Utilities|Array|Random (Variables|/n00dFootsteps/Core/PDA_N00dFootstepsSurface.PDA_N00dFootstepsSurface_C|GetWaves (N00d|Footsteps|Casting|ConverttoDefaultSurface PrimaryData)))))
    (:Completed
      (bind _assound_base (Utilities|Casting|CastToSoundBase _object))
      (bind _returnvalue (Audio|SpawnSoundatLocation _assound_base Location "0, 0, 0" _volume 1.0 0.0 0 0))
      (Utilities|IsValid _returnvalue
        (:Is%20Valid
          ;[1 1 1] Bind to completed audio
          (Variables|UI|SetVolumeDisplay (Utilities|Text|ToText(Float) _volume "HalfToEven"))
          (Variables|UI|SetSpeedDisplay (Utilities|Text|ToText(Float) _speed "HalfToEven"))
          (EventDispatchers|BindEventtoOnAudioFinished _returnvalue (EventDispatchers|CreateEvent :!event Custom|FootstepAudioFinished))
          ;[1 1 1] Add the incoming and show the int we've added
          (bind _returnvalue_2 (Utilities|Array|Add (Variables|Reference|GetActiveAudioComponents) 0))
          (Variables|UI|SetActiveAudioDisplay (Utilities|Text|ToText(Integer) _returnvalue_2)))))))

(event Custom|FootstepAudioFinished
  (bind _activeaudiocomponents (Variables|Reference|GetActiveAudioComponents))
  ;[1 1 1] Audio finished
  ;;[1 1 1] Remove a sound and debug the active sounds
  (Utilities|Array|RemoveIndex _activeaudiocomponents)
  (Variables|UI|SetActiveAudioDisplay (Utilities|Text|ToText(Integer) (Utilities|Array|Length _activeaudiocomponents))))

(event EventBeginPlay
  ;[1 1 1] Destroy self if we are disabled (we are created automatically, so remove what we don't need)
  (if (N00d|Footsteps|System|IsDisabled)
    (Components|DestroyComponent)
    (else
      (N00d|Footsteps|System|Load))))

(fn Footstep
  (params (Data :type FN00d%20Footstep%20Bone%20Data%20Structure))
  (bind _footprintdata (Variables|Defaults|GetFootprintData))
  (bind _currentfootprint (Variables|Reference|GetCurrentFootprint))
  (bind _foleydata (Variables|Defaults|GetFoleyData))
  (LocalVariables|SetLocalData Data)
  (Utilities|FlowControl|Sequence
    (:then_0
      ;[1 1 1] Cache the owning character's socket world transform
      (bind _output_get (LocalVariables|SetLocalMesh (Variables|/Script/Engine.Character|GetMesh (N00d|Footsteps|System|GetOwningCharacter))))
      (LocalVariables|SetLocalTransform (Transformation|GetSocketTransform _output_get (.foot (LocalVariables|GetLocalData)) "RTS_World")))
    (:then_1
      ;[1 1 1] Trace from the bone's world transform and apply the delta and offset
      (bind (_outhit _returnvalue) (Collision|LineTraceForObjects (Math|Vector|MakeVector (.X (Math|Vector|BreakVector (Math|Vector|MakeVector (.x (.location (LocalVariables|GetLocalTransform))) (.y (.location (LocalVariables|GetLocalTransform))) (+ (.z (.location (LocalVariables|GetLocalTransform))) (.offset (LocalVariables|GetLocalData)))))) (.Y (Math|Vector|BreakVector (Math|Vector|MakeVector (.x (.location (LocalVariables|GetLocalTransform))) (.y (.location (LocalVariables|GetLocalTransform))) (+ (.z (.location (LocalVariables|GetLocalTransform))) (.offset (LocalVariables|GetLocalData)))))) (- (.Z (Math|Vector|BreakVector (Math|Vector|MakeVector (.x (.location (LocalVariables|GetLocalTransform))) (.y (.location (LocalVariables|GetLocalTransform))) (+ (.z (.location (LocalVariables|GetLocalTransform))) (.offset (LocalVariables|GetLocalData)))))) (.delta (LocalVariables|GetLocalData)))) (Math|Vector|MakeVector (.X (Math|Vector|BreakVector (Math|Vector|MakeVector (.x (.location (LocalVariables|GetLocalTransform))) (.y (.location (LocalVariables|GetLocalTransform))) (+ (.z (.location (LocalVariables|GetLocalTransform))) (.offset (LocalVariables|GetLocalData)))))) (.Y (Math|Vector|BreakVector (Math|Vector|MakeVector (.x (.location (LocalVariables|GetLocalTransform))) (.y (.location (LocalVariables|GetLocalTransform))) (+ (.z (.location (LocalVariables|GetLocalTransform))) (.offset (LocalVariables|GetLocalData)))))) (+ (.Z (Math|Vector|BreakVector (Math|Vector|MakeVector (.x (.location (LocalVariables|GetLocalTransform))) (.y (.location (LocalVariables|GetLocalTransform))) (+ (.z (.location (LocalVariables|GetLocalTransform))) (.offset (LocalVariables|GetLocalData)))))) (.delta (LocalVariables|GetLocalData)))) (Variables|Defaults|GetObjectTypes) (Variables|Defaults|GetTraceComplex) 0 (select (N00d|Footsteps|System|IsDebug) "ForDuration" "None")))
      (bind _output_get_2 (LocalVariables|SetLocalHit _returnvalue))
      (if _output_get_2
        ;[1 1 1] Cache the current surface data
        (LocalVariables|SetLocalSurface (N00d|Footsteps|Casting|ConvertSurfaceTypetoData (Variables|/Script/PhysicsCore.PhysicalMaterial|GetSurfaceType (.PhysMat (Collision|BreakHitResult _outhit)))))
        (LocalVariables|SetLocalLocation (.Location (Collision|BreakHitResult _outhit)))
        (Variables|UI|SetSurfaceDisplay (Utilities|Text|ToText(String) (Utilities|String|EnumtoString (Variables|/Script/PhysicsCore.PhysicalMaterial|GetSurfaceType (.PhysMat (Collision|BreakHitResult _outhit))))))
        (bind _output_get_3 (Variables|Reference|SetHitActor (.HitActor (Collision|BreakHitResult _outhit))))
        (Variables|UI|SetActorDisplay (Utilities|Text|ToText(String) (Utilities|GetDisplayName _output_get_3)))
        (else
          (N00d|Footsteps|System|Debug "MISSED GROUND" "(R=1.000000,G=1.000000,B=0.000000,A=1.000000)"))))
    (:then_2
      ;[1 1 1] Spawn the effect
      (if (LocalVariables|GetLocalHit)
        (if (Utilities|IsValidSoftObjectReference (Variables|/n00dFootsteps/Core/PDA_N00dFootstepsSurface.PDA_N00dFootstepsSurface_C|GetNiagaraEffect (N00d|Footsteps|Casting|ConverttoDefaultSurface (LocalVariables|GetLocalSurface))))
          (CallFunction|SpawnNiagara (LocalVariables|GetLocalLocation) (LocalVariables|GetLocalSurface))
          (elif (Utilities|IsValidSoftObjectReference (Variables|/n00dFootsteps/Core/PDA_N00dFootstepsSurface.PDA_N00dFootstepsSurface_C|GetCascadeEffect (N00d|Footsteps|Casting|ConverttoDefaultSurface (LocalVariables|GetLocalSurface))))
            (CallFunction|SpawnCascade (LocalVariables|GetLocalLocation) (LocalVariables|GetLocalSurface))
            (else
              (N00d|Footsteps|System|Debug "NO EFFECTS DEFINED FOR THIS SURFACE!" "(R=1.000000,G=0.000000,B=0.000000,A=1.000000)"))))))
    (:then_3
      ;[1 1 1] Spawn sound
      (if (LocalVariables|GetLocalHit)
        (if (Utilities|Array|IsValidIndex (Variables|/n00dFootsteps/Core/PDA_N00dFootstepsSurface.PDA_N00dFootstepsSurface_C|GetWaves (N00d|Footsteps|Casting|ConverttoDefaultSurface (LocalVariables|GetLocalSurface))))
          (CallFunction|SpawnAudio (LocalVariables|GetLocalLocation) (LocalVariables|GetLocalSurface))
          (else
            (N00d|Footsteps|System|Debug "NO AUDIO DEFINED FOR THIS SURFACE!" "(R=1.000000,G=0.000000,B=0.000000,A=1.000000)")))))
    (:then_4
      ;[1 1 1] Spawn a footprint
      (if (LocalVariables|GetLocalHit)
        (if (Variables|/n00dFootsteps/Core/PDA_N00dFootstepsSurface.PDA_N00dFootstepsSurface_C|GetLeavesFootprint (N00d|Footsteps|Casting|ConverttoDefaultSurface (LocalVariables|GetLocalSurface)))
          (if (Utilities|Array|IsValidIndex _footprintdata)
            (for _array_element _footprintdata
              (if (== (Variables|/n00dFootsteps/Core/PDA_N00dFootprint.PDA_N00dFootprint_C|GetTag (N00d|Footsteps|Casting|ConverttoDefaultFootprint _array_element)) (select (GameplayTags|IsGameplayTagValid _currentfootprint) _currentfootprint (Variables|Defaults|GetDefaultFootprint)))
                (CallFunction|SpawnFootprint (select (.left (LocalVariables|GetLocalData)) (Variables|/n00dFootsteps/Core/PDA_N00dFootprint.PDA_N00dFootprint_C|GetLeftFoot (N00d|Footsteps|Casting|ConverttoDefaultFootprint _array_element)) (Variables|/n00dFootsteps/Core/PDA_N00dFootprint.PDA_N00dFootprint_C|GetRightFoot (N00d|Footsteps|Casting|ConverttoDefaultFootprint _array_element))) (LocalVariables|GetLocalLocation) (Variables|/n00dFootsteps/Core/PDA_N00dFootstepsSurface.PDA_N00dFootstepsSurface_C|GetFootprintTint (N00d|Footsteps|Casting|ConverttoDefaultSurface (LocalVariables|GetLocalSurface))))
                (Variables|UI|SetFootDisplay (select (.left (LocalVariables|GetLocalData)) "Left Foot" "Right Foot"))))
            (else
              (N00d|Footsteps|System|Debug "NO FOOTPRINTS DEFINED!" "(R=1.000000,G=0.000000,B=0.000000,A=1.000000)"))))))
    (:then_5
      ;[1 1 1] Spawn foley sound
      (if (and (LocalVariables|GetLocalHit) (Utilities|Array|IsValidIndex _foleydata))
        (bind _array_element_2 (Utilities|Array|ForEachLoopwithBreak _foleydata :!label _label)
          (:LoopBody
            (if (== (select (GameplayTags|IsGameplayTagValid (Variables|Reference|GetCurrentFoley)) (Variables|Reference|GetCurrentFoley) (Variables|Defaults|GetDefaultFoley)) (Variables|/n00dFootsteps/Core/PDA_N00dFootstepsFoley.PDA_N00dFootstepsFoley_C|GetTag (N00d|Footsteps|Casting|ConverttoDefaultFoley _array_element_2)))
              (if (Utilities|Array|IsValidIndex (Variables|/n00dFootsteps/Core/PDA_N00dFootstepsFoley.PDA_N00dFootstepsFoley_C|GetWaves (N00d|Footsteps|Casting|ConverttoDefaultFoley _array_element_2)))
                (CallFunction|SpawnFoley (LocalVariables|GetLocalLocation) (N00d|Footsteps|Casting|ConverttoDefaultFoley _array_element_2))
                (goto _label Break)
                (else
                  (N00d|Footsteps|System|Debug "NO FOLEY DEFINED FOR THIS TAG!" "(R=1.000000,G=0.000000,B=0.000000,A=1.000000)")
                  (goto _label Break))))))))))

(fn Load
  (bind _owningcharacter (N00d|Footsteps|System|GetOwningCharacter))
  (bind _defaultfoley (Variables|Defaults|GetDefaultFoley))
  (bind _returnvalue (Pawn|GetController _owningcharacter))
  ;[1 1 1] Cache the owning character
  (bind _ascharacter (Utilities|Casting|CastToCharacter (Components|GetOwner)))
  (Variables|Reference|SetOwningCharacter _ascharacter)
  ;[1 1 1] Debug
  ;;[1 1 1] Are we debugging
  (if (N00d|Footsteps|System|IsDebug)
    ;;[1 1 1] Get the owning character's player controller and add the debug widget to the screen
    (if (Pawn|IsLocallyControlled _owningcharacter)
      (if (Pawn|IsLocalPlayerController _returnvalue)
        (bind _asplayer_controller (Utilities|Casting|CastToPlayerController _returnvalue))
        (bind _returnvalue_2 (UserInterface|CreateWidget "/n00dFootsteps/Core/WBP_N00dFootstepsDebug.WBP_N00dFootstepsDebug_C" _asplayer_controller))
        (UserInterface|Viewport|AddtoViewport _returnvalue_2 0)
        ;;[1 1 1] Default footprint
        (Variables|UI|SetFootprintDisplay (Utilities|Text|ToText(Name) (GameplayTags|GetTagName (Variables|Defaults|GetDefaultFootprint))))
        ;;[1 1 1] Default foley
        (Variables|UI|SetFoleyDisplay (select (GameplayTags|IsGameplayTagValid _defaultfoley) (Utilities|Text|ToText(Name) (GameplayTags|GetTagName _defaultfoley)) "Undefined"))))))

(fn IsDebug
  (return (or (Variables|Defaults|GetDebugFootsteps) (Variables|/Script/n00dFootsteps.N00dFootstepsSettings|GetDebugFootsteps (Class|N00dFootstepsSettings|GetFootstepsSettings)))))

(fn IsDisabled
  (return (or (Variables|Defaults|GetDisableFootsteps) (Variables|/Script/n00dFootsteps.N00dFootstepsSettings|GetDisableFootsteps (Class|N00dFootstepsSettings|GetFootstepsSettings)))))

(fn GetOwningCharacter
  (return (Variables|Reference|GetOwningCharacter)))

(fn ConvertSurfaceTypetoData
  (params (SurfaceType :type EPhysicalSurface%20Enum :default "SurfaceType_Default"))
  ;[1 1 1] Scan the array for the surface type from the default primary data asset and return it
  (bind _array_element (Utilities|Array|ForEachLoopwithBreak (Variables|Defaults|GetSurfaceData) :!label _label)
    (:LoopBody
      (if (Utilities|Enum|Equal(Enum) (Variables|/n00dFootsteps/Core/PDA_N00dFootstepsSurface.PDA_N00dFootstepsSurface_C|GetSurfaceType (N00d|Footsteps|Casting|ConverttoDefaultSurface _array_element)) SurfaceType)
        (LocalVariables|SetLocalData _array_element)
        (goto _label Break)))
    (:Completed
      (return (LocalVariables|GetLocalData)))))

(fn ConverttoDefaultSurface
  (params (PrimaryData :type Primary%20Data%20Asset%20Object%20Reference))
  (bind _asn00dfootsteps_surface_data (Utilities|Casting|CastToPDA_N00dFootstepsSurface PrimaryData))
  (return _asn00dfootsteps_surface_data))

(fn Debug
  (params (InString :type String) (TextColor :type Linear%20Color%20Structure :default "(R=0.000000,G=0.660000,B=1.000000,A=1.000000)"))
  (if (N00d|Footsteps|System|IsDebug)
    (Development|PrintString (Utilities|String|Append "(n00dFootsteps): " InString) true true TextColor))
  (return))

(fn ConverttoDefaultFootprint
  (params (Current :type Primary%20Data%20Asset%20Object%20Reference))
  (bind _aspda_n00d_footprint (Utilities|Casting|CastToPDA_N00dFootprint Current))
  (return _aspda_n00d_footprint))

(fn SetFootprint
  (params (Footprint :type Gameplay%20Tag%20Structure))
  (Variables|Reference|SetCurrentFootprint Footprint))

(fn GetVolume
  (bind _owningcharacter (N00d|Footsteps|System|GetOwningCharacter))
  (bind _returnvalue (Transformation|GetVelocity _owningcharacter))
  (bind _returnvalue_2 (Math|Vector|VectorLength _returnvalue))
  ;[1 1 1] Normalise to a default volume multiplier range
  (return (Math|Float|NormalizetoRange (/ _returnvalue_2 (Class|MovementComponent|GetMaxSpeed (Variables|/Script/Engine.Character|GetCharacterMovement _owningcharacter))) 0.0 1.0) _returnvalue_2))

(fn ConverttoDefaultFoley
  (params (Current :type Primary%20Data%20Asset%20Object%20Reference))
  (bind _aspda_n00d_footsteps_foley (Utilities|Casting|CastToPDA_N00dFootstepsFoley Current))
  (return _aspda_n00d_footsteps_foley))

(fn SetFoley
  (params (Foley :type Gameplay%20Tag%20Structure))
  (Variables|Reference|SetCurrentFoley Foley))