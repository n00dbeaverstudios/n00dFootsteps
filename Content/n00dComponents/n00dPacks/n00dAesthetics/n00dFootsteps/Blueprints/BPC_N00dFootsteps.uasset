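; Footstep component that plays surface-based sounds, particles and decals for actors, pawns or characters, driven by movement axis input or anim notify sockets.
; Surface type comes from socket or actor line traces or the CharacterMovement floor hit, with configurable trace complexity.
; It feeds a master cue wave, foley, rattle, gender and volume parameters, with foley and rattle chosen by armour type.
; Axis footsteps route through the server and multicast to clients.
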(event Custom|ServerPlayAxisFootsteps
  ;[0.1903 0.6116 0.705] Networking
  ;;[1 0.05 0.05] Send important tasks to the server for Axis replication
  (N00dComponents|Footsteps|Checks|SwitchonAxisComplexity))

(event Custom|MulticastSpawnFX
  ;[0.1903 0.6116 0.705] Networking
  ;;[1 0.05 0.05] Multicast the FX for all clients to see the Axis footstep replication
  (N00dComponents|Footsteps|Effects|SpawnFX))

(event Custom|MulticastSelectSound
  ;[0.1903 0.6116 0.705] Networking
  ;;[1 0.05 0.05] Multicast the FX for all clients to see the Axis footstep replication
  (N00dComponents|Footsteps|Sounds|SelectSound))

(event EventSetArmourType
  (params (ArmourType :type EN00dFootstepsArmourTypes%20Enum :default "NewEnumerator0"))
  ;[1 1 1] INFO
  ;;[1 1 1] Send in custom variables from other BPs to determine automatic handling of certain sounds.
  ;;
  ;; Walking type will affect rattle and armour type will affect foley. You can implement your own interface and replace these for your own custom enums if need be
  (Variables|N00dComponents|Footsteps|DoNotEdit|SetArmourType ArmourType))

(event EventSetWalkingType
  ;[1 1 1] INFO
  ;;[1 1 1] Send in custom variables from other BPs to determine automatic handling of certain sounds.
  ;;
  ;; Walking type will affect rattle and armour type will affect foley. You can implement your own interface and replace these for your own custom enums if need be
)

(fn PlayAxisFootsteps
  (params (Axis :type Float%20%28single-precision%29))
  (bind _owningpawn (Variables|Default|GetOwningPawn))
  ;[1 1 1] Handle the networking of the Axis footsteps and send it off for processing on the server
  ;;[1 1 1] Make sure our incoming axis is in range of our defined values as to not always be ticking
  (if (N00dComponents|Footsteps|Checks|FootstepsShouldPlayAxis Axis)
    ;;[1 1 1] Don't do anything if we're coming in on a notify for whatever reason
    (switch Utilities|FlowControl|Switch|SwitchonEN00dFootstepPlayType (Variables|N00dComponents|Footsteps|Config|Defaults|GetFootstepPlayType)
      (:NewEnumerator0
        ;;[1 1 1] Check if we're the server after validating our pawn
        (Utilities|IsValid _owningpawn
          (:Is%20Valid
            (if (Ability|HasAuthority (Pawn|GetController _owningpawn))
              ;;[1 1 1] Handle switching defaults for OnAxis settings
              (N00dComponents|Footsteps|Checks|SwitchonAxisComplexity)
              (return) ; Go home. Wifey was proud
              (else
                ;;[1 1 1] Send the remote to the server
                (CallFunction|ServerPlayAxisFootsteps)
                (return) ; Do a round trip, bruh. You forgot the milk
              )))
          (:Is%20Not%20Valid
            (return))))
      (:NewEnumerator1
        (return) ; Why you playin' with me
      ))
    (else
      (return) ; Let's save some processing
    )))

(fn MovementIsinRange
  (params (Axis :type Float%20%28single-precision%29))
  ;[1 1 1] Adjust these values in the class defaults to be as sensitive as required
  (if (or (Math|Float|InRange(Float) Axis (Variables|N00dComponents|Footsteps|Config|Axis|GetNegativeMin) (Variables|N00dComponents|Footsteps|Config|Axis|GetNegativeMax)) (Math|Float|InRange(Float) Axis (Variables|N00dComponents|Footsteps|Config|Axis|GetPositiveMin) (Variables|N00dComponents|Footsteps|Config|Axis|GetPositiveMax)))
    (return true)
    (else
      (return false))))

(fn FootstepsShouldPlayAxis
  (params (Axis :type Float%20%28single-precision%29))
  (bind _owningcmc (Variables|Default|GetOwningCMC))
  ;[1 1 1] Return true if we meet the conditions
  (Utilities|IsValid _owningcmc
    (:Is%20Valid
      (return (and (N00dComponents|Footsteps|Checks|MovementIsinRange Axis) (not (AI|Components|NavMovement|IsFalling _owningcmc)))))
    (:Is%20Not%20Valid
      (return false))))

(fn SelectSound
  ;[1 1 1] Select and play our sound according to the play type and trace complexity
  ;;[1 1 1] Set our conditions on entry
  (switch Utilities|FlowControl|Switch|SwitchonEN00dFootstepPlayType (Variables|N00dComponents|Footsteps|Config|Defaults|GetFootstepPlayType)
    (:NewEnumerator0
      (Variables|N00dComponents|Footsteps|DoNotEdit|SetIgnoreIsPlaying false))
    (:NewEnumerator1
      (switch Utilities|FlowControl|Switch|SwitchonEN00dTraceComplexity (Variables|N00dComponents|Footsteps|Config|Defaults|GetTraceComplexity)
        (:NewEnumerator0
          (Variables|N00dComponents|Footsteps|DoNotEdit|SetIgnoreIsPlaying false :!label _label))
        (:NewEnumerator4
          (goto _label))
        (:NewEnumerator1
          (Variables|N00dComponents|Footsteps|DoNotEdit|SetIgnoreIsPlaying true)))))
  ;;[1 1 1] Should we not ignore the IsPlaying flag
  (if (not (Variables|N00dComponents|Footsteps|DoNotEdit|GetIgnoreIsPlaying))
    ;;[1 1 1] Handle Footstep Sounds
    ;;;[1 1 1] Check that there's at least one AudioComponent and that it's not playing... if not, spawn one
    (Utilities|IsValid (Variables|N00dComponents|Footsteps|DoNotEdit|GetPrimaryAudioComponent)
      (:Is%20Valid
        (if (Audio|Components|Audio|IsPlaying (Variables|N00dComponents|Footsteps|DoNotEdit|GetPrimaryAudioComponent))
          (return)
          (else
            _)))
      (:Is%20Not%20Valid
        _))
    ;;;[1 1 1] Spawn FX for intermittent
    (N00dComponents|Footsteps|Effects|SpawnIntermittentFX))
  ;;;[1 1 1] Spawn a component at the actor's location
  (bind _returnvalue (Audio|SpawnSoundatLocation (N00dComponents|Footsteps|Sounds|GetFootstepsSoundsforSurface) (Transformation|GetActorLocation (Components|GetOwner))))
  (Variables|N00dComponents|Footsteps|DoNotEdit|SetPrimaryAudioComponent _returnvalue)
  ;;;[1 1 1] Set our master cue parameters each time we fire
  (N00dComponents|Footsteps|Sounds|SetMasterCueParameters)
  (return))

(fn GetFootstepsSoundsforSurface
  (bind _masterfootstep (Variables|N00dComponents|Footsteps|Config|Defaults|GetMasterFootstep))
  (bind _footsteps (Variables|N00dComponents|Footsteps|Config|Defaults|GetFootsteps))
  (bind _currentsurfacetype (Variables|N00dComponents|Footsteps|DoNotEdit|GetCurrentSurfaceType))
  (bind _value (Utilities|Map|Find _footsteps _currentsurfacetype))
  (bind _sound (Utilities|Struct|BreakFN00dFootstepEffects _value))
  ;[1 1 1] If the default is invalid, pull from our footsteps map
  (Utilities|IsValid _masterfootstep
    (:Is%20Valid
      (return _masterfootstep))
    (:Is%20Not%20Valid
      (Utilities|IsValid _sound
        (:Is%20Valid
          (return _sound))
        (:Is%20Not%20Valid
          (return 0))))))

(fn PlayNotifyFootsteps
  (params (SocketName :type Name))
  (switch Utilities|FlowControl|Switch|SwitchonEN00dFootstepPlayType (Variables|N00dComponents|Footsteps|Config|Defaults|GetFootstepPlayType)
    (:NewEnumerator0
      (return))
    (:NewEnumerator1
      ;[1 1 1] Store the defined socket for use in the trace
      (Variables|N00dComponents|Footsteps|DoNotEdit|SetCurrentSocket SocketName)
      (switch Utilities|FlowControl|Switch|SwitchonEN00dTraceComplexity (Variables|N00dComponents|Footsteps|Config|Defaults|GetTraceComplexity)
        (:NewEnumerator0
          (return))
        (:NewEnumerator4
          ;[1 1 1] Intermittent Notify trace
          ;;[1 1 1] Find the trace and set the FX
          (N00dComponents|Footsteps|Trace|SetSurfaceType true)
          (N00dComponents|Footsteps|Sounds|SelectSound)
          ;;[1 1 1] DEBUG Current Surface Type
          (CallFunction|Debug (Utilities|String|EnumtoString (Variables|N00dComponents|Footsteps|DoNotEdit|GetCurrentSurfaceType)) "NewEnumerator1" "PhysMat:" (Variables|Default|GetWidgetPrinting) false 0.0)
          (return))
        (:NewEnumerator1
          ;[1 1 1] Attached Notify Trace
          ;;[1 1 1] Trace and store the relevant returned results
          (N00dComponents|Footsteps|Trace|SetSurfaceTypeFX true)
          ;;[1 1 1] DEBUG Current Surface Type
          (CallFunction|Debug (Utilities|String|EnumtoString (Variables|N00dComponents|Footsteps|DoNotEdit|GetCurrentSurfaceType)) "NewEnumerator1" "PhysMat:" (Variables|Default|GetWidgetPrinting) false 1e+01)
          (return))))))

(fn SpawnFX
  (bind _footsteps (Variables|N00dComponents|Footsteps|Config|Defaults|GetFootsteps))
  (bind _currentsurfacetype (Variables|N00dComponents|Footsteps|DoNotEdit|GetCurrentSurfaceType))
  (bind _value (Utilities|Map|Find _footsteps _currentsurfacetype))
  (bind (_particleeffects _particlematerial _decal) (Utilities|Struct|BreakFN00dFootstepEffects _value))
  ;[1 1 1] Spawn all the FX. All of them.
  ;;[1 1 1] Handle setting surface type and FX on intermittent (ie if this is executed from a notify)
  (switch Utilities|FlowControl|Switch|SwitchonEN00dTraceComplexity (Variables|N00dComponents|Footsteps|Config|Defaults|GetTraceComplexity)
    (:NewEnumerator0
      _)
    (:NewEnumerator4
      (N00dComponents|Footsteps|Trace|SetSurfaceTypeFX true))
    (:NewEnumerator1
      _))
  (Utilities|FlowControl|Sequence
    (:then_0
      ;;[1 1 1] Handle spawning our relevant effects
      ;;;[1 1 1] Handle playing sounds
      (N00dComponents|Footsteps|Sounds|SelectSound))
    (:then_1
      ;;;[1 1 1] Handle spawning the particles
      (N00dComponents|Footsteps|Effects|SpawnParticle _particleeffects _particlematerial))
    (:then_2
      ;;;[1 1 1] Handle Decals
      (N00dComponents|Footsteps|Effects|SpawnDecal _decal))
    (:then_3
      (return))))

(fn GetRandomWave
  (params (Array :type Array%20of%20Sound%20Wave%20Object%20References))
  (bind _returnvalue (Utilities|Array|Length Array))
  (bind _returnvalue_2 (Math|Random|RandomInteger _returnvalue))
  (if (Utilities|Array|IsValidIndex Array _returnvalue_2)
    (return (Utilities|Array|Get(acopy) Array _returnvalue_2))
    (else
      (return 0))))

(fn GetSurfaceTypeWaves
  (return (Utilities|Struct|BreakFN00dArrayOfWaves (.Value (Utilities|Map|Find (.SurfaceTypeWaves (Utilities|Struct|BreakFN00dFootstepParameters (Variables|N00dComponents|Footsteps|Config|Defaults|GetSoundParameters))) (Variables|N00dComponents|Footsteps|DoNotEdit|GetCurrentSurfaceType))))))

(fn SetMasterCueParameters
  (bind _soundparameters (Variables|N00dComponents|Footsteps|Config|Defaults|GetSoundParameters))
  (bind (_shouldrattle _rattlewaves _shouldfoley _foleywaves _ismale) (Utilities|Struct|BreakFN00dFootstepParameters _soundparameters))
  ;[1 1 1] Set master CUE parameters
  (Utilities|IsValid (Variables|N00dComponents|Footsteps|DoNotEdit|GetPrimaryAudioComponent)
    (:Is%20Valid
      ;;[1 1 1] Set random wave inside the Master CUE
      ;;;[1 1 1] Get Random Footstep Wave from Current SurfaceType
      (Class|AudioComponent|SetWaveParameter (Variables|N00dComponents|Footsteps|DoNotEdit|GetPrimaryAudioComponent) "SurfaceType" (N00dComponents|Footsteps|Sounds|GetRandomWave (N00dComponents|Footsteps|Sounds|GetSurfaceTypeWaves)))
      ;;[1 1 1] Set parameters in the MasterFootstepsCUE
      (|SetRattle _shouldrattle _rattlewaves)
      (|SetFoley _shouldfoley _foleywaves)
      (|SetGender _ismale)
      (Audio|Components|Audio|AdjustVolume)
      (|ModifyAttenuation)
      (return))
    (:Is%20Not%20Valid
      (return))))

(fn SetSurfaceTypeFX
  (params (Simple :type Boolean))
  (LocalVariables|SetLocalSimple Simple)
  ;[1 1 1] Switch on ActorType
  (switch Utilities|FlowControl|Switch|SwitchonEN00dFootstepActorType (Variables|N00dComponents|Footsteps|Config|Defaults|GetActorType)
    (:NewEnumerator0
      _)
    (:NewEnumerator1
      _)
    (:NewEnumerator2
      ;[1 1 1] Switch on Character Trace Type
      (switch Utilities|FlowControl|Switch|SwitchonEN00dFootstepCharacterTrace (Variables|N00dComponents|Footsteps|Config|Defaults|GetCharacterTraceType)
        (:NewEnumerator1
          ;[1 1 1] Mesh trace
          ;;[1 1 1] Set surface type
          (bind _meshvalid (N00dComponents|Footsteps|Trace|SetSurfaceTypefromMesh (LocalVariables|GetLocalSimple)))
          (if _meshvalid
            ;;[1 1 1] Play the FX
            (N00dComponents|Footsteps|Effects|SpawnFX)
            (return)
            (else
              _)))
        (:NewEnumerator0
          ;[1 1 1] Character Movement Component Trace
          ;;[1 1 1] IMPORTANT: you MUST set the CapsuleComponent in the character to ReturnMaterialOnMove for this to work!
          (N00dComponents|Footsteps|Trace|SetSurfaceTypefromCMC)
          ;;[1 1 1] Play the FX
          (N00dComponents|Footsteps|Effects|SpawnFX)
          (return)))))
  ;[1 1 1] Actor Trace
  ;;[1 1 1] Set surface type
  (N00dComponents|Footsteps|Trace|SetSurfaceTypefromActorLocation (LocalVariables|GetLocalSimple))
  ;;[1 1 1] Play the FX
  (N00dComponents|Footsteps|Effects|SpawnFX)
  (return))

(fn TraceforSurfaceType
  (params (Start :type Vector) (End :type Vector) (Simple :type Boolean))
  ;[1 1 1] Trace from defined start point to end point, store the hit, and get the surface type
  (bind (_outhit _returnvalue) (Collision|LineTraceByChannel Start End (Variables|N00dComponents|Footsteps|Config|Tracing|GetTraceChannel) (not Simple) (Utilities|Array|MakeArray (Variables|Default|GetOwningCharacter)) (Variables|N00dComponents|Footsteps|Config|Tracing|GetDrawDebugType)))
  (if _returnvalue
    (bind _output_get (Variables|N00dComponents|Footsteps|DoNotEdit|SetCurrentHit _outhit))
    (return (Variables|/Script/Engine.PhysicalMaterial|GetSurfaceType (.PhysMat (Collision|BreakHitResult _output_get))))
    (else
      (return "SurfaceType_Default"))))

(fn GetRelevantSpawnLocation
  (bind _returnvalue (Components|GetOwner))
  (bind _returnvalue_2 (Components|GetOwner))
  (bind _offsetfx (Variables|N00dComponents|Footsteps|Config|Axis|GetOffsetFX))
  (bind _owningcharacter (Variables|Default|GetOwningCharacter))
  (bind _actortype (Variables|N00dComponents|Footsteps|Config|Defaults|GetActorType))
  (bind _offsetfx_2 (Variables|N00dComponents|Footsteps|Config|Axis|GetOffsetFX))
  (bind _returnvalue_3 (Transformation|GetActorLocation _returnvalue_2))
  (bind _returnvalue_4 (Transformation|GetActorLocation _returnvalue))
  (bind _mesh (Variables|/Script/Engine.Character|GetMesh _owningcharacter))
  (bind _returnvalue_5 (Transformation|GetSocketLocation _mesh "root"))
  (bind _returnvalue_6 (+ _returnvalue_4 _offsetfx))
  (bind _returnvalue_7 (+ _returnvalue_3 _offsetfx_2))
  (bind _returnvalue_8 (Utilities|Select :Index _actortype :NewEnumerator0 _returnvalue_7 :NewEnumerator1 _returnvalue_7 :NewEnumerator2 _returnvalue_5))
  ;[1 1 1] Make sure the owning character is valid if we're that actor type
  (switch Utilities|FlowControl|Switch|SwitchonEN00dFootstepActorType (Variables|N00dComponents|Footsteps|Config|Defaults|GetActorType)
    (:NewEnumerator0
      _)
    (:NewEnumerator1
      _)
    (:NewEnumerator2
      (Utilities|IsValid (Variables|Default|GetOwningCharacter)
        (:Is%20Valid
          _)
        (:Is%20Not%20Valid
          (return "0, 0, 0")))))
  (return (Utilities|Select :Index (Variables|N00dComponents|Footsteps|Config|Defaults|GetFootstepPlayType) :NewEnumerator0 (Utilities|Select :Index (Variables|N00dComponents|Footsteps|Config|Defaults|GetTraceComplexity) :NewEnumerator0 "0, 0, 0" :NewEnumerator4 _returnvalue_8 :NewEnumerator1 _returnvalue_8) :NewEnumerator1 (Utilities|Select :Index (Variables|N00dComponents|Footsteps|Config|Defaults|GetActorType) :NewEnumerator0 _returnvalue_6 :NewEnumerator1 _returnvalue_6 :NewEnumerator2 (Utilities|Select :Index (Variables|N00dComponents|Footsteps|Config|Defaults|GetCharacterTraceType) :NewEnumerator1 (Transformation|GetSocketLocation (Variables|/Script/Engine.Character|GetMesh (Variables|Default|GetOwningCharacter)) (Variables|N00dComponents|Footsteps|DoNotEdit|GetCurrentSocket)) :NewEnumerator0 _returnvalue_6)))))

(fn SpawnParticle
  (params (ParticleSystem :type Particle%20System%20Object%20Reference) (ParticleMaterial :type Material%20Interface%20Object%20Reference))
  (Utilities|IsValid ParticleSystem
    (:Is%20Valid
      ;[1 1 1] Spawn a template emitter and set its material, if none valid, return
      (bind _returnvalue (Effects|SpawnEmitteratLocation ParticleSystem (N00dComponents|Footsteps|Effects|GetRelevantSpawnLocation)))
      (Utilities|IsValid ParticleMaterial
        (:Is%20Valid
          (Rendering|Material|SetMaterial _returnvalue 0 ParticleMaterial)
          (return))
        (:Is%20Not%20Valid
          (return))))
    (:Is%20Not%20Valid
      (return))))

(fn SpawnDecal
  (params (FootstepDecal :type FN00d%20Footstep%20Decals%20Structure%20%28by%20ref%29))
  (bind (_decalmaterial _feetdecals) (Utilities|Struct|BreakFN00dFootstepDecals FootstepDecal))
  (bind _currentsocket (Variables|N00dComponents|Footsteps|DoNotEdit|GetCurrentSocket))
  (bind _returnvalue (Utilities|String|ToString(Name) _currentsocket))
  ;[1 1 1] Spawn Decals
  ;;[1 1 1] Cache incoming
  (LocalVariables|SetLocalDecal FootstepDecal)
  (LocalVariables|SetLocalPrimaryDecal _decalmaterial)
  (LocalVariables|SetLocalFeetDecals _feetdecals)
  ;;[1 1 1] Is our primary decal valid
  (Utilities|IsValid (LocalVariables|GetLocalPrimaryDecal)
    (:Is%20Valid
      _)
    (:Is%20Not%20Valid
      ;;[1 1 1] If the primary decal material is empty, lets find the corresponding socket and flag it accordingly
      (if (Utilities|String|Contains _returnvalue (Utilities|String|ToString(Name) (.LeftFootSocket (Utilities|Struct|BreakFN00dFootstepsFeet (LocalVariables|GetLocalFeetDecals)))))
        (LocalVariables|SetLocalLeft true)
        (elif (Utilities|String|Contains _returnvalue (Utilities|String|ToString(Name) (.RightFootSocket (Utilities|Struct|BreakFN00dFootstepsFeet (LocalVariables|GetLocalFeetDecals)))))
          (LocalVariables|SetLocalLeft false)))
      ;;[1 1 1] Get the decal for the current surface left or right foot and spawn it according to our defined settings
      (Utilities|IsValid (.LeftFoot (Utilities|Struct|BreakFN00dFootstepsFeet (LocalVariables|GetLocalFeetDecals)))
        (:Is%20Valid
          _)
        (:Is%20Not%20Valid
          (Utilities|IsValid (.RightFoot (Utilities|Struct|BreakFN00dFootstepsFeet (LocalVariables|GetLocalFeetDecals)))
            (:Is%20Valid
              _)
            (:Is%20Not%20Valid
              (return)))))))
  ;;[1 1 1] Spawn the decal with defined defaults
  (bind _returnvalue_2 (Rendering|Decal|SpawnDecalatLocation (select (Utilities|IsValid (LocalVariables|GetLocalPrimaryDecal)) (LocalVariables|GetLocalPrimaryDecal) (select (LocalVariables|GetLocalLeft) (.LeftFoot (Utilities|Struct|BreakFN00dFootstepsFeet (LocalVariables|GetLocalFeetDecals))) (.RightFoot (Utilities|Struct|BreakFN00dFootstepsFeet (LocalVariables|GetLocalFeetDecals))))) (.ReturnValue (N00dComponents|Footsteps|Effects|GetDecalDefaults (LocalVariables|GetLocalDecal))) (.ImpactPoint (N00dComponents|Footsteps|Effects|GetDecalDefaults (LocalVariables|GetLocalDecal))) (.Rotation (N00dComponents|Footsteps|Effects|GetDecalDefaults (LocalVariables|GetLocalDecal))) (.Lifetime (N00dComponents|Footsteps|Effects|GetDecalDefaults (LocalVariables|GetLocalDecal)))))
  ;;[0.2462 0.323 0.34] DEBUG
  (CallFunction|Debug (Utilities|GetDisplayName _returnvalue_2) "NewEnumerator1" "DECAL:" false false 0.0))

(fn SpawnIntermittentFX
  (bind _footsteps (Variables|N00dComponents|Footsteps|Config|Defaults|GetFootsteps))
  (bind _currentsurfacetype (Variables|N00dComponents|Footsteps|DoNotEdit|GetCurrentSurfaceType))
  (bind _value (Utilities|Map|Find _footsteps _currentsurfacetype))
  (bind (_particleeffects _particlematerial _decal) (Utilities|Struct|BreakFN00dFootstepEffects _value))
  ;[1 1 1] Same as SpawnFX just without SelectSound as we are firing this function from within SelectSound
  (switch Utilities|FlowControl|Switch|SwitchonEN00dTraceComplexity (Variables|N00dComponents|Footsteps|Config|Defaults|GetTraceComplexity)
    (:NewEnumerator0
      (return))
    (:NewEnumerator4
      (Utilities|FlowControl|Sequence
        (:then_0
          ;;[1 1 1] Handle spawning our relevant intermittent effects
          ;;;[1 1 1] Handle spawning the particles
          (N00dComponents|Footsteps|Effects|SpawnParticle _particleeffects _particlematerial))
        (:then_1
          ;;;[1 1 1] Handle Decals
          (N00dComponents|Footsteps|Effects|SpawnDecal _decal))
        (:then_2
          (return))))
    (:NewEnumerator1
      (return))))

(fn SetSurfaceTypefromCMC
  (bind _owningcmc (Variables|Default|GetOwningCMC))
  (bind _currentfloor (Variables|/Script/Engine.CharacterMovementComponent|GetCurrentFloor _owningcmc))
  (bind (_bwalkablefloor _hitresult) (Utilities|Struct|BreakFindFloorResult _currentfloor))
  (bind _physmat (Collision|BreakHitResult _hitresult))
  ;[1 1 1] Get surface type
  ;;[1 1 1] Return if the floor is not walkable
  (if _bwalkablefloor
    ;;[1 1 1] Set the CurrentSurfaceType
    (Utilities|IsValid _physmat
      (:Is%20Valid
        (Variables|N00dComponents|Footsteps|DoNotEdit|SetCurrentSurfaceType (Variables|/Script/Engine.PhysicalMaterial|GetSurfaceType _physmat)))
      (:Is%20Not%20Valid
        (Variables|N00dComponents|Footsteps|DoNotEdit|SetCurrentSurfaceType "SurfaceType_Default")))
    (return)
    (else
      (return))))

(fn SetSurfaceTypefromMesh
  (params (Simple :type Boolean))
  (bind _currentsocket (Variables|N00dComponents|Footsteps|DoNotEdit|GetCurrentSocket))
  (bind _owningcharacter (Variables|Default|GetOwningCharacter))
  (bind _notifytracepoints (Variables|N00dComponents|Footsteps|Config|Tracing|GetNotifyTracePoints))
  (bind _mesh (Variables|/Script/Engine.Character|GetMesh _owningcharacter))
  (bind _returnvalue (Transformation|GetSocketLocation _mesh _currentsocket))
  ;[1 1 1] Trace from the incoming current socket location (e.g. foot socket from anim notify) and store the CurrentSurfaceType
  ;;[1 1 1] Validate Character
  (Utilities|IsValid _owningcharacter
    (:Is%20Valid
      ;;[1 1 1] Character Mesh defined socket location and Z offset, if not valid find actor location, if we have a mesh
      (Utilities|IsValid _mesh
        (:Is%20Valid
          ;;[1 1 1] Trace for Surface
          (bind _surfacetype (N00dComponents|Footsteps|Trace|TraceforSurfaceType (+ _returnvalue (Math|Vector|MakeVector 0.0 0.0 (.x _notifytracepoints))) (+ _returnvalue (Math|Vector|MakeVector 0.0 0.0 (.y _notifytracepoints))) Simple))
          (Variables|N00dComponents|Footsteps|DoNotEdit|SetCurrentSurfaceType _surfacetype)
          (return true))
        (:Is%20Not%20Valid
          ;;[0.2462 0.323 0.34] Debug
          (CallFunction|Debug "Owning Character Mesh NOT VALID - CharacterMesh not Applied?" "NewEnumerator4" "DECAL:" false false 0.0)
          (return false))))
    (:Is%20Not%20Valid
      (return false))))

(fn SetSurfaceTypefromActorLocation
  (params (Simple :type Boolean))
  (bind _returnvalue (Components|GetOwner))
  (bind _actortracepoints (Variables|N00dComponents|Footsteps|Config|Tracing|GetActorTracePoints))
  (bind _returnvalue_2 (Transformation|GetActorLocation _returnvalue))
  ;[1 1 1] Custom Trace for surface type
  (bind _surfacetype (N00dComponents|Footsteps|Trace|TraceforSurfaceType (+ _returnvalue_2 (.start _actortracepoints)) (+ _returnvalue_2 (.end _actortracepoints)) Simple))
  (Variables|N00dComponents|Footsteps|DoNotEdit|SetCurrentSurfaceType _surfacetype)
  (return))

(fn SetSurfaceType
  (params (Simple :type Boolean))
  ;[1 1 1] Set our relevant surface type according to the actor we are attached to
  (LocalVariables|SetLocalSimple Simple)
  ;;[1 1 1] Switch on ActorType
  (switch Utilities|FlowControl|Switch|SwitchonEN00dFootstepActorType (Variables|N00dComponents|Footsteps|Config|Defaults|GetActorType)
    (:NewEnumerator0
      _)
    (:NewEnumerator1
      _)
    (:NewEnumerator2
      ;;[1 1 1] Switch on Character Trace Type
      (switch Utilities|FlowControl|Switch|SwitchonEN00dFootstepCharacterTrace (Variables|N00dComponents|Footsteps|Config|Defaults|GetCharacterTraceType)
        (:NewEnumerator1
          ;;[1 1 1] Mesh trace
          ;;;[1 1 1] Set surface type
          (bind _meshvalid (N00dComponents|Footsteps|Trace|SetSurfaceTypefromMesh (LocalVariables|GetLocalSimple)))
          (if _meshvalid
            (return)
            (else
              _)))
        (:NewEnumerator0
          ;;[1 1 1] Character Movement Component Trace
          ;;;[1 1 1] IMPORTANT: you MUST set the CapsuleComponent in the character to ReturnMaterialOnMove for this to work!
          (N00dComponents|Footsteps|Trace|SetSurfaceTypefromCMC)
          (return)))))
  ;;[1 1 1] Actor Trace
  ;;;[1 1 1] Set surface type
  (N00dComponents|Footsteps|Trace|SetSurfaceTypefromActorLocation (LocalVariables|GetLocalSimple))
  (return))

(fn GetDecalDefaults
  (params (Decal :type FN00d%20Footstep%20Decals%20Structure))
  (bind (_decalmaterial _feetdecals _size _lifetime _addtox _addtoy) (Utilities|Struct|BreakFN00dFootstepDecals Decal))
  (bind _returnvalue (Components|GetOwner))
  (bind _actortype (Variables|N00dComponents|Footsteps|Config|Defaults|GetActorType))
  (bind _owningcharacter (Variables|Default|GetOwningCharacter))
  (bind _returnvalue_2 (Utilities|Select :Index _actortype :NewEnumerator0 _returnvalue :NewEnumerator1 _returnvalue :NewEnumerator2 _owningcharacter))
  (bind _returnvalue_3 (Transformation|GetActorRotation _returnvalue_2))
  ;[1 1 1] Cache
  (Utilities|IsValid (Variables|Default|GetOwningCharacter)
    (:Is%20Valid
      (LocalVariables|SetLocalSize _size)
      (LocalVariables|SetLocalLifetime _lifetime)
      (LocalVariables|SetLocalAddToX _addtox)
      (LocalVariables|SetLocalAddToY _addtoy)
      (return (* "1.000000,1.000000,1.000000" (LocalVariables|GetLocalSize)) (.ImpactPoint (Collision|BreakHitResult (Variables|N00dComponents|Footsteps|DoNotEdit|GetCurrentHit))) (Math|Rotator|MakeRotator (+ (.roll _returnvalue_3) (LocalVariables|GetLocalAddToX)) (+ (.pitch _returnvalue_3) (LocalVariables|GetLocalAddToY)) (.yaw _returnvalue_3)) (LocalVariables|GetLocalLifetime)))
    (:Is%20Not%20Valid
      (return "0, 0, 0" "0, 0, 0" "0, 0, 0" 0.0))))

(fn SwitchonAxisComplexity
  ;[1 1 1] Footstep types
  ;;[1 1 1] Switch on Complexity
  (switch Utilities|FlowControl|Switch|SwitchonEN00dTraceComplexity (Variables|N00dComponents|Footsteps|Config|Defaults|GetTraceComplexity)
    (:NewEnumerator0
      ;;[1 1 1] Basic Constant Audio - this will play only when movement occurs
      ;;;[1 1 1] Play footstep sounds
      (N00dComponents|Footsteps|Effects|SpawnFX)
      ;;;[1 1 1] Send the effects to all clients
      (CallFunction|MulticastSpawnFX)
      ;;;[1 1 1] DEBUG Play
      (CallFunction|Debug (Utilities|GetDisplayName (Variables|N00dComponents|Footsteps|DoNotEdit|GetPrimaryAudioComponent)) "NewEnumerator1" "Playing" (Variables|Default|GetWidgetPrinting) false 0.0)
      (return))
    (:NewEnumerator4
      ;;[1 1 1] Intermittently Handled Single Persistent Trace
      ;;;[1 1 1] Find the trace and set the FX
      (N00dComponents|Footsteps|Trace|SetSurfaceType true)
      (N00dComponents|Footsteps|Sounds|SelectSound)
      ;;;[1 1 1] Send the effects to all clients
      (CallFunction|MulticastSelectSound)
      ;;;[1 1 1] DEBUG Current Surface Type
      (CallFunction|Debug (Utilities|String|EnumtoString (Variables|N00dComponents|Footsteps|DoNotEdit|GetCurrentSurfaceType)) "NewEnumerator1" "PhysMat:" (Variables|Default|GetWidgetPrinting) false 0.0)
      (return))
    (:NewEnumerator1
      ;;[1 1 1] Simple Single Persistent Trace
      ;;;[1 1 1] Trace and store the relevant returned results
      (N00dComponents|Footsteps|Trace|SetSurfaceTypeFX true)
      ;;;[1 1 1] Send the effects to all clients
      (CallFunction|MulticastSpawnFX)
      ;;;[1 1 1] DEBUG Current Surface Type
      (CallFunction|Debug (Utilities|String|EnumtoString (Variables|N00dComponents|Footsteps|DoNotEdit|GetCurrentSurfaceType)) "NewEnumerator1" "PhysMat:" (Variables|Default|GetWidgetPrinting) false 0.0)
      (return))))

(fn GetFootstepsComponent
  (return 0))